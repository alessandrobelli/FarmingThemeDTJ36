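; BP_CropBase is a crop actor that grows toward harvest, needs periodic watering and withers if neglected.
; Chained timers drive its state from planting through water calls to harvest-ready or withered, and watering restarts the water cycle.
; Tick turns timer values into a widget countdown bar and three mesh growth stages.
; A dynamic material hue shift signals thirst and withering, and interacting with a withered crop destroys it.
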(event `SetDMIHue`
  (params (Hue :type "Float (double-precision)"))
  (bind _output_get (set `self.CurrentHue` Hue))
  (bind _cropmaterialdmi (`self.CropMaterialDMI`)
    (:`then`
      (`MaterialInstanceDynamic.SetScalarParameterValue` _cropmaterialdmi "RandomHue Shift" _output_get))
    (:`else`)))

(event `SetDynamicMaterial`
  (bind _crop (`self.Crop`))
  (bind _returnvalue (`PrimitiveComponent.CreateDynamicMaterialInstance` _crop 0 (`PrimitiveComponent.GetMaterial` _crop 0) "None"))
  (set `self.CropMaterialDMI` _returnvalue)
  (bind _cropmaterialdmi (`self.CropMaterialDMI`)
    (:`then`
      (`MaterialInstanceDynamic.SetScalarParameterValue` _cropmaterialdmi "RandomHue Shift" (`self.CurrentHue`)))
    (:`else`)))

(event `self.ReceiveBeginPlay`
  ;[1 0 0 0.5] BeginPlay
  (set `self.CurrentCropState` "NewEnumerator0")
  (`self.ClearTimers`)
  (bind _aswbp_crop_timer_ui (cast `/Game/UI/WBP_CropTimerUI` (`WidgetComponent.GetUserWidgetObject` (`self.CropTimerWidgetComponent`)))
    (:`then`
      (set `self.CropTimerUI_Ref` _aswbp_crop_timer_ui))
    (:`CastFailed`
      _))
  (`self.StartTimers`)
  (bind _returnvalue (`KismetSystemLibrary.K2_SetTimerDelegate` (delegate `OnReadyToHarvest`) (`self.GrowthToHarvestDuration`)))
  (set `self.TimerHandle_GrowthToHarvest` _returnvalue)
  (`StaticMeshComponent.SetStaticMesh` (`self.Crop`) (`|GetArrayItem` (`self.GrowthStageMeshes`)))
  (set `self.CurrentHue` 0.0)
  (`self.SetDynamicMaterial`))

(event `OnReadyToHarvest`
  (`KismetSystemLibrary.PrintString` "ready to harvest")
  (if (`|EnumInequality` (`self.CurrentCropState`) "NewEnumerator4")
    (set `self.CurrentCropState` "NewEnumerator3")
    (`self.ClearTimers`)
    (bind _returnvalue (`KismetSystemLibrary.K2_SetTimerDelegate` (delegate `OnSpoiled`)))
    (set `self.TimerHandle_Wither` _returnvalue)))

(event `OnSpoiled`
  (set `self.CurrentCropState` "NewEnumerator4"))

(event `StartTimers`
  (bind _returnvalue (`KismetSystemLibrary.K2_SetTimerDelegate` (delegate `TransitionToNeedsWater`) (`self.TimeUntilFirstWaterCallDuration`)))
  (set `self.TimerHandle_WaterCall` _returnvalue))

(event `TransitionToNeedsWater`
  (`KismetSystemLibrary.K2_ClearAndInvalidateTimerHandle` (`self.TimerHandle_WaterCall`))
  (`self.SetDMIHue` 0.5)
  (set `self.CurrentCropState` "NewEnumerator2")
  (bind _returnvalue (`KismetSystemLibrary.K2_SetTimerDelegate` (delegate `TransitionToWithered`) (`self.WaterWindowBeforeWitherDuration`)))
  (set `self.TimerHandle_Wither` _returnvalue))

(event `ClearTimers`
  (`KismetSystemLibrary.K2_ClearAndInvalidateTimerHandle` (`self.TimerHandle_WaterCall`))
  (`KismetSystemLibrary.K2_ClearAndInvalidateTimerHandle` (`self.TimerHandle_Wither`)))

(event `TransitionToWithered`
  (`self.SetDMIHue` 0.6)
  (set `self.CurrentCropState` "NewEnumerator4")
  (`self.ClearTimers`)
  (`KismetSystemLibrary.PrintString` "Withered")
  (`KismetSystemLibrary.K2_ClearAndInvalidateTimerHandle` (`self.TimerHandle_GrowthToHarvest`)))

(event `PlayerInteracted_Water`
  (`GameplayStatics.PlaySound2D` "/Game/Sounds/watering.watering" 0.5 (`KismetMathLibrary.RandomFloatInRange` 0.9 1.2) 0.0 "/Game/Sounds/SC_Watering.SC_Watering" (`GameplayStatics.GetPlayerPawn` 0) false)
  (`KismetSystemLibrary.PrintString` "watering")
  (set `self.CurrentCropState` "NewEnumerator1")
  (`self.ClearTimers`)
  (`self.StartTimers`)
  (`self.SetDMIHue` 0.0))

(event `PlayerInteracted_Withered`
  (if (`|EnumEquality` (`self.CurrentCropState`) "NewEnumerator4")
    (`self.K2_DestroyActor`)))

(event `self.ReceiveTick`
  (params (DeltaSeconds :type "Float (single-precision)"))
  (bind _growthtoharvestduration (`self.GrowthToHarvestDuration`))
  (bind _growthstagemeshes (`self.GrowthStageMeshes`))
  (bind _timerhandle_wither (`self.TimerHandle_Wither`))
  (bind _timerhandle_watercall (`self.TimerHandle_WaterCall`))
  (bind _croptimerui_ref (`self.CropTimerUI_Ref`))
  (bind _timerhandle_growthtoharvest (`self.TimerHandle_GrowthToHarvest`))
  (bind _returnvalue (+ (`self.TimeUntilFirstWaterCallDuration`) (`self.WaterWindowBeforeWitherDuration`)))
  (bind _returnvalue_2 (`KismetMathLibrary.Clamp` (`KismetMathLibrary.FFloor` (/ (`KismetSystemLibrary.K2_GetTimerElapsedTimeHandle` _timerhandle_growthtoharvest) (/ _growthtoharvestduration 3.0))) 0 2))
  (switch `/Game/E_CropStates` (`self.CurrentCropState`)
    (:`NewEnumerator0`
      (if (`KismetSystemLibrary.K2_IsValidTimerHandle` _timerhandle_watercall) :!label _label
        (bind _output_get (set `self.CalculatedOverallRemainingTime` (+ (`KismetSystemLibrary.K2_GetTimerRemainingTimeHandle` _timerhandle_watercall) (`self.WaterWindowBeforeWitherDuration`))))
        (bind _output_get_2 (set `self.FillPercentage` (/ _output_get _returnvalue)))
        (`/Game/UI/WBP_CropTimerUI.UpdateFillPercent` _croptimerui_ref (`KismetMathLibrary.FClamp` _output_get_2))
        (if (`KismetSystemLibrary.K2_IsTimerActiveHandle` _timerhandle_growthtoharvest) :!label _label_2
          (if (> _growthtoharvestduration 0.0)
            (if (not (== _returnvalue_2 (`self.CurrentVisualStage`)))
              (bind _output_get_3 (set `self.CurrentVisualStage` _returnvalue_2))
              (if (`KismetArrayLibrary.Array_IsValidIndex` _growthstagemeshes _output_get_3)
                (`StaticMeshComponent.SetStaticMesh` (`self.Crop`) (`|GetArrayItem` _growthstagemeshes _output_get_3))
                (`self.SetDynamicMaterial`)))))
        (elif (`KismetSystemLibrary.K2_IsTimerActiveHandle` _timerhandle_wither)
          (bind _output_get_4 (set `self.CalculatedOverallRemainingTime` (`KismetSystemLibrary.K2_GetTimerRemainingTimeHandle` _timerhandle_wither)))
          (bind _output_get_5 (set `self.FillPercentage` (/ _output_get_4 _returnvalue)))
          (`/Game/UI/WBP_CropTimerUI.UpdateFillPercent` _croptimerui_ref (`KismetMathLibrary.FClamp` _output_get_5))
          (goto _label_2)
          (else
            (set `self.CalculatedOverallRemainingTime` _returnvalue)))))
    (:`NewEnumerator1`
      (goto _label))
    (:`NewEnumerator2`
      (goto _label))
    (:`NewEnumerator3`
      (`Widget.SetVisibility` (`/Game/UI/WBP_CropTimerUI.ProgressBar` (`self.CropTimerUI_Ref`)) "Hidden"))))

(fn `UserConstructionScript`)